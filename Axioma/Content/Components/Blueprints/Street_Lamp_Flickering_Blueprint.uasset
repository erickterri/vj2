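; Street lamp Blueprint that makes its spot light flicker irregularly.
; Tick drives a chain of four random-length Delay nodes, each followed by a visibility toggle on the SpotLight and its child components.
; Tick re-enters the chain every frame, so the flicker repeats continuously without an explicit loop or timer.
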(event `self.ReceiveTick`
  (params (DeltaSeconds :type "Float (single-precision)"))
  (`KismetSystemLibrary.Delay` (`KismetMathLibrary.RandomFloatInRange` 0.5 1.5))
  (`SceneComponent.ToggleVisibility` (`self.SpotLight`) true)
  (`KismetSystemLibrary.Delay` (`KismetMathLibrary.RandomFloatInRange` 0.0 0.5))
  (`SceneComponent.ToggleVisibility` (`self.SpotLight`) true)
  (`KismetSystemLibrary.Delay` (`KismetMathLibrary.RandomFloatInRange` 0.1 1.0))
  (`SceneComponent.ToggleVisibility` (`self.SpotLight`) true)
  (`KismetSystemLibrary.Delay` (`KismetMathLibrary.RandomFloatInRange` 0.0 0.2))
  (`SceneComponent.ToggleVisibility` (`self.SpotLight`) true))

(fn `UserConstructionScript`)