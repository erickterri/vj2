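; Defective traffic light Blueprint that blinks its green light for as long as it runs.
; BeginPlay toggles GreenLight visibility every half second through a Delay that loops back on itself.
; GoToNextState defines a Red, Green, Yellow cycle that also switches the walk lights on Red and Green.
; The looping timer that would drive that cycle is disconnected, so the state machine does not run from this graph.
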(event `/Game/Components/Blueprints/Traffic_Light_Normal_Blueprint.ReceiveBeginPlay`
  (for _ (range 1) :!label _label
    (`SceneComponent.ToggleVisibility` (`self.GreenLight`) false)
    (`KismetSystemLibrary.Delay` 0.5)
    (goto _label)))

(fn `GoToNextState`
  (bind _greenlight (`self.GreenLight`))
  (bind _yellowlight (`self.YellowLight`))
  (bind _redlight (`self.RedLight`))
  (bind _redwalklight (`self.RedWalkLight`))
  (bind _greenwalklight (`self.GreenWalkLight`))
  (switch `/Game/Components/Blueprints/TrafficEnum` (`self.State`)
    (:`NewEnumerator0`
      (set `self.State` "NewEnumerator3")
      (`SceneComponent.SetVisibility` _redlight false false)
      (`SceneComponent.SetVisibility` _yellowlight false false)
      (`SceneComponent.SetVisibility` _greenlight true false)
      (`SceneComponent.SetVisibility` _redwalklight true false)
      (`SceneComponent.SetVisibility` _greenwalklight false false))
    (:`NewEnumerator2`
      (set `self.State` "NewEnumerator0")
      (`SceneComponent.SetVisibility` _redlight true false)
      (`SceneComponent.SetVisibility` _yellowlight false false)
      (`SceneComponent.SetVisibility` _greenlight false false)
      (`SceneComponent.SetVisibility` _redwalklight false false)
      (`SceneComponent.SetVisibility` _greenwalklight true false))
    (:`NewEnumerator3`
      (set `self.State` "NewEnumerator2")
      (`SceneComponent.SetVisibility` _redlight false false)
      (`SceneComponent.SetVisibility` _yellowlight true false)
      (`SceneComponent.SetVisibility` _greenlight false false))))

(fn `UserConstructionScript`)