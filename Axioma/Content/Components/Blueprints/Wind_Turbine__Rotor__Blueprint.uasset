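; Wind turbine rotor Blueprint that spins its Rotor component continuously.
; Tick adds a small random world-space roll each frame without delta-time scaling, so the spin varies slightly and depends on frame rate.
; The construction script gives the rotor a random relative pitch between 0 and 180 degrees, then prints a separately evaluated random value, which need not match that pitch.
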(event `self.ReceiveTick`
  (params (DeltaSeconds :type "Float (single-precision)"))
  (`SceneComponent.K2_AddWorldRotation` (`self.Rotor`) (`KismetMathLibrary.MakeRotator` (`KismetMathLibrary.RandomFloatInRange` 0.5 1.0)) false false))

(fn `UserConstructionScript`
  (bind _returnvalue (`KismetMathLibrary.RandomFloatInRange` 0.0 180.0))
  (`SceneComponent.K2_SetRelativeRotation` (`self.Rotor`) (`KismetMathLibrary.MakeRotator` 0.0 _returnvalue) false false)
  (`KismetSystemLibrary.PrintString` (`KismetStringLibrary.Conv_DoubleToString` _returnvalue)))