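; Traffic light Blueprint that cycles Green, Yellow and Red vehicle lights along with red and green pedestrian walk lights.
; BeginPlay loops endlessly, calling GoToNextState, then waiting three times the new state's Delay value.
; GoToNextState advances State and toggles light component visibility; walk lights switch only on entering Green or Red.
; A looping timer call to GoToNextState is present but unconnected.
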(event `self.ReceiveBeginPlay`
  (for _ (range 1) :!label _label
    (`self.GoToNextState`)
    (switch `/Game/Components/Blueprints/TrafficEnum` (`self.State`)
      (:`NewEnumerator0`
        (bind _output_get (set `self.Delay` 3.0)))
      (:`NewEnumerator2`
        (bind _output_get_2 (set `self.Delay` 1.0)))
      (:`NewEnumerator3`
        (bind _output_get_3 (set `self.Delay` 4.0))))
    (`KismetSystemLibrary.Delay` (+ _output_get _output_get_2 _output_get_3))
    (goto _label)))

(fn `GoToNextState`
  (bind _greenlight (`self.GreenLight`))
  (bind _yellowlight (`self.YellowLight`))
  (bind _redlight (`self.RedLight`))
  (bind _redwalklight (`self.RedWalkLight`))
  (bind _greenwalklight (`self.GreenWalkLight`))
  (switch `/Game/Components/Blueprints/TrafficEnum` (`self.State`)
    (:`NewEnumerator0`
      (set `self.State` "NewEnumerator3")
      (`SceneComponent.SetVisibility` _redlight false false)
      (`SceneComponent.SetVisibility` _yellowlight false false)
      (`SceneComponent.SetVisibility` _greenlight true false)
      (`SceneComponent.SetVisibility` _redwalklight true false)
      (`SceneComponent.SetVisibility` _greenwalklight false false))
    (:`NewEnumerator2`
      (set `self.State` "NewEnumerator0")
      (`SceneComponent.SetVisibility` _redlight true false)
      (`SceneComponent.SetVisibility` _yellowlight false false)
      (`SceneComponent.SetVisibility` _greenlight false false)
      (`SceneComponent.SetVisibility` _redwalklight false false)
      (`SceneComponent.SetVisibility` _greenwalklight true false))
    (:`NewEnumerator3`
      (set `self.State` "NewEnumerator2")
      (`SceneComponent.SetVisibility` _redlight false false)
      (`SceneComponent.SetVisibility` _yellowlight true false)
      (`SceneComponent.SetVisibility` _greenlight false false))))

(fn `UserConstructionScript`)